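; Prototype launch pad actor that throws characters and static mesh actors upward and along the pad's facing when they overlap it.
; On overlap, characters receive LaunchCharacter with a velocity built from the pad rotation's X axis plus a fixed upward boost.
; Static mesh actors instead get a similarly directed AddForce as an acceleration change, then a debug print shows the direction vector.
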(event `self.ReceiveActorBeginOverlap`
  (params (OtherActor :type "Actor Object Reference"))
  (bind _x (.x (`KismetMathLibrary.BreakRotIntoAxes` (`self.K2_GetActorRotation`))))
  (bind _y (.y (`KismetMathLibrary.BreakRotIntoAxes` (`self.K2_GetActorRotation`))))
  (bind _ascharacter (cast `Character` OtherActor)
    (:`then`
      (`Character.LaunchCharacter` _ascharacter (`KismetMathLibrary.MakeVector` (* _x 400.0) (* _y 400.0) 1000.0) false false))
    (:`CastFailed`
      (bind _asstatic_mesh_actor (cast `StaticMeshActor` OtherActor))
      (`PrimitiveComponent.AddForce` (`StaticMeshActor.StaticMeshComponent` _asstatic_mesh_actor) (`KismetMathLibrary.MakeVector` (* _x 50000.0) (* _y 50000.0) 200000.0) "None" true)
      (`KismetSystemLibrary.PrintString` (`KismetTextLibrary.Conv_TextToString` (`|FormatText` "x={x} y={y} z={z}" _x _y (.z (`KismetMathLibrary.BreakRotIntoAxes` (`self.K2_GetActorRotation`)))))))))

(fn `UserConstructionScript`)